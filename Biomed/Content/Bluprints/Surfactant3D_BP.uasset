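; Surfactant3D actor whose physics sphere wanders randomly along the world axes until it overlaps something.
; While not arrived, Tick uses a Delay to periodically set an axis-aligned velocity, re-rolling the random number for each of six directions.
; Overlap sets ActorArrived, zeroes velocity and suspends gravity for a timed period; end overlap resumes wandering.
; BeginPlay only delays, and the looping movement and collision-change events are not called here.
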(event `GoToRandomPosition`
  (bind _returnvalue (`KismetMathLibrary.RandomIntegerInRange` 1 6))
  (bind _speedmaximum (`self.SpeedMaximum`))
  (bind _returnvalue_2 (* _speedmaximum -1.0))
  ;[0.364 0.2355 1] Go To a random Position
  (`|ExecutionSequence`
    (:`then_0`
      (if (== _returnvalue 1)
        (set `self.Speed` (`KismetMathLibrary.MakeVector` _speedmaximum))
        (`PrimitiveComponent.SetPhysicsLinearVelocity` (`self.Sphere`) (`self.Speed`) false "None" :!label _label)))
    (:`then_1`
      (if (== _returnvalue 2)
        (set `self.Speed` (`KismetMathLibrary.MakeVector` _returnvalue_2))
        (goto _label)))
    (:`then_2`
      (if (== _returnvalue 3)
        (set `self.Speed` (`KismetMathLibrary.MakeVector` 0.0 _speedmaximum))
        (goto _label)))
    (:`then_3`
      (if (== _returnvalue 4)
        (set `self.Speed` (`KismetMathLibrary.MakeVector` 0.0 _returnvalue_2))
        (goto _label)))
    (:`then_4`
      (if (== _returnvalue 5)
        (set `self.Speed` (`KismetMathLibrary.MakeVector` 0.0 0.0 _speedmaximum))
        (goto _label)))
    (:`then_5`
      (if (== _returnvalue 6)
        (set `self.Speed` (`KismetMathLibrary.MakeVector` 0.0 0.0 _returnvalue_2))
        (goto _label)))))

(event `KeepGoingToArandomPostition`
  ;[1 1 1] GoingToRandomPositionEvent
  (`self.GoToRandomPosition` :!label _label_2)
  (`KismetSystemLibrary.Delay` 0.1)
  (if (not (`self.Actor Arrived?`))
    (goto _label_2)))

(event `SetSpeedToZero`
  (bind _sphere (`self.Sphere`))
  ;[0.8031 0.3051 1] Setting Speed To Zero
  (`PrimitiveComponent.SetPhysicsLinearVelocity` _sphere (0.0 0.0 0.0) false "None")
  (`PrimitiveComponent.SetPhysicsAngularVelocityInDegrees` _sphere (0.0 0.0 0.0) false "None"))

(event `self.ReceiveTick`
  (params (DeltaSeconds :type "Float (single-precision)"))
  ;[0.9583 0.1312 0] TickEvent
  (if (`self.Actor Arrived?`)
    (`self.SetSpeedToZero`)
    (else
      (`KismetSystemLibrary.Delay` 0.2)
      (`self.GoToRandomPosition`))))

(event `self.Sphere.OnComponentBeginOverlap`
  (params (OverlappedComponent :type "PrimitiveComponent Object Reference") (OtherActor :type "Actor Object Reference") (OtherComp :type "PrimitiveComponent Object Reference") (OtherBodyIndex :type Integer) (bFromSweep :type Boolean) (SweepResult :type "HitResult Structure (by ref)"))
  ;[1 1 1] OverlappingEvent
  (set `self.Actor Arrived?` true)
  (`self.SetSpeedToZero`)
  (`PrimitiveComponent.SetEnableGravity` (`self.Sphere`) false)
  (`KismetSystemLibrary.Delay` 20.0)
  (`PrimitiveComponent.SetEnableGravity` (`self.Sphere`) true))

(event `self.Sphere.OnComponentEndOverlap`
  (params (OverlappedComponent :type "PrimitiveComponent Object Reference") (OtherActor :type "Actor Object Reference") (OtherComp :type "PrimitiveComponent Object Reference") (OtherBodyIndex :type Integer))
  ;[1 1 1] EndOverlapEvent
  (set `self.Actor Arrived?` false))

(event `self.ReceiveBeginPlay`
  ;[1 1 1] TheBeginPlay
  (`KismetSystemLibrary.Delay` 10.0))

(event `ChangeCollision`
  ;[1 1 1] Changing Collision
  (`PrimitiveComponent.SetCollisionResponseToChannel` (`self.Sphere`) "ECC_PhysicsBody" "ECR_Block"))

(fn `UserConstructionScript`)